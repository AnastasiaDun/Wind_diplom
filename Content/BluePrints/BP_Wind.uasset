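; BP_Wind is a moving wind actor that travels along its arrow direction and steers around obstacles.
; Each tick it traces from three points, stepping forward on clear traces and yawing via two angled probes when blocked.
; When it hits another BP_Wind, it snaps to their combined heading and eases the other around with a timeline.
; Box overlaps send activate messages with wind strength, and deactivate on exit.
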(event OnComponentBeginOverlap(Sphere1)
  (params (OverlappedComponent :type Primitive%20Component%20Object%20Reference) (OtherActor :type Actor%20Object%20Reference) (OtherComp :type Primitive%20Component%20Object%20Reference) (OtherBodyIndex :type Integer) (bFromSweep :type Boolean) (SweepResult :type Hit%20Result%20Structure%20%28by%20ref%29)))

(event OnComponentEndOverlap(Sphere1)
  (params (OverlappedComponent :type Primitive%20Component%20Object%20Reference) (OtherActor :type Actor%20Object%20Reference) (OtherComp :type Primitive%20Component%20Object%20Reference) (OtherBodyIndex :type Integer)))

(event OnComponentBeginOverlap(Box1)
  (params (OverlappedComponent :type Primitive%20Component%20Object%20Reference) (OtherActor :type Actor%20Object%20Reference) (OtherComp :type Primitive%20Component%20Object%20Reference) (OtherBodyIndex :type Integer) (bFromSweep :type Boolean) (SweepResult :type Hit%20Result%20Structure%20%28by%20ref%29))
  (Class|WindInterface|Activate(Message) OtherActor self (Variables|Default|GetWindStrength)))

(event OnComponentEndOverlap(Box1)
  (params (OverlappedComponent :type Primitive%20Component%20Object%20Reference) (OtherActor :type Actor%20Object%20Reference) (OtherComp :type Primitive%20Component%20Object%20Reference) (OtherBodyIndex :type Integer))
  (Class|WindInterface|Deactivate(Message) OtherActor))

(event Custom|Rotation
  (params (Arrow :type Arrow%20Component%20Object%20Reference))
  (Variables|Default|SetNewVar_1 (Transformation|GetActorRotation self))
  (Variables|Default|SetNewVar_0 (Math|Conversions|RotationFromXVector (+ (Math|Vector|GetForwardVector Arrow) (Math|Vector|GetForwardVector (Variables|Default|GetArrow)))))
  (bind _newtrack_0 (Timeline|Timeline_0 PlayFromStart)
    (:Update
      (Transformation|SetActorRotation self (Math|Rotator|Lerp(Rotator) (Variables|Default|GetNewVar_1) (Variables|Default|GetNewVar_0) _newtrack_0)))))

(event Custom|RotateSelf
  (params (Actor :type Actor%20Object%20Reference))
  (bind _asbp_wind (Utilities|Casting|CastToBP_Wind Actor))
  (CallFunction|Rotation _asbp_wind (Variables|Default|GetArrow))
  (Variables|Default|SetNewVar_2 (Math|Conversions|RotationFromXVector (+ (Math|Vector|GetForwardVector (Variables|BP_Wind_C|GetArrow _asbp_wind)) (Math|Vector|GetForwardVector (Variables|Default|GetArrow)))))
  (Variables|Default|SetNewVar_3 (Transformation|GetActorRotation self))
  (bind _newtrack_0 (Timeline|Timeline_2 PlayFromStart)
    (:Update
      (Transformation|SetActorRotation self (Math|Rotator|Lerp(Rotator) (Variables|Default|GetNewVar_3) (Variables|Default|GetNewVar_2) _newtrack_0)))))

(event EventBeginPlay
  (if (Variables|Default|GetDebug)
    (Components|Sphere|SetSphereRadius (Variables|Default|GetSphere1) (Variables|Default|GetIn%20Sphere%20Radius) true)
    (else
      (Components|DestroyComponent (Variables|Default|GetSphere1)))))

(event EventTick
  (params (DeltaSeconds :type Float%20%28single-precision%29))
  (Utilities|FlowControl|Sequence
    (:then_0
      (CallFunction|CeckPregrada (Variables|Default|GetSphere) (Variables|Default|GetArrow)))
    (:then_1
      (CallFunction|CeckPregrada (Variables|Default|GetSphere2) (Variables|Default|GetArrow1)))
    (:then_2
      (CallFunction|CeckPregrada (Variables|Default|GetSphere3) (Variables|Default|GetArrow2)))))

(fn ConstructionScript
  (Components|Sphere|SetSphereRadius (Variables|Default|GetSphere1) (Variables|Default|GetIn%20Sphere%20Radius) true))

(fn CeckPregrada
  (params (Start :type Static%20Mesh%20Component%20Object%20Reference) (End :type Arrow%20Component%20Object%20Reference))
  (bind _returnvalue (Transformation|GetWorldLocation Start))
  (bind _self self)
  (bind _self_2 self)
  (bind _self_3 self)
  (bind _returnvalue_2 (Transformation|GetWorldLocation Start))
  (bind _returnvalue_3 (Transformation|GetWorldLocation Start))
  (bind _returnvalue_4 (Transformation|GetActorRotation _self_3))
  (bind _returnvalue_5 (Transformation|GetActorRotation _self_2))
  (Utilities|IsValid Start
    (:Is%20Valid
      (Utilities|IsValid End
        (:Is%20Valid
          (bind (_outhit _returnvalue_6) (Collision|LineTraceForObjects _returnvalue (+ _returnvalue (* (Math|Vector|GetForwardVector End) (Variables|Default|GetDistanse))) (Utilities|Array|MakeArray "ObjectTypeQuery1" "ObjectTypeQuery2" "ObjectTypeQuery4") false 0 "None"))
          (if _returnvalue_6
            (if (== (Utilities|GetClass (.hitactor _outhit)) "BP_Wind_C")
              (bind _output_get (Variables|Default|SetOut%20Hit%20Hit%20Actor (.hitactor _outhit)))
              (bind _asbp_wind (Utilities|Casting|CastToBP_Wind _output_get))
              (if (not (Math|Rotator|Equal(Rotator) (Transformation|GetActorRotation _self) (Math|Conversions|RotationFromXVector (+ (Math|Vector|GetForwardVector (Variables|BP_Wind_C|GetArrow _asbp_wind)) (Math|Vector|GetForwardVector (Variables|Default|GetArrow)))) 0.1))
                (Transformation|SetActorRotation _self (Math|Conversions|RotationFromXVector (+ (Math|Vector|GetForwardVector (Variables|BP_Wind_C|GetArrow _asbp_wind)) (Math|Vector|GetForwardVector (Variables|Default|GetArrow)))))
                (CallFunction|Rotation _asbp_wind (Variables|Default|GetArrow)))
              (else
                (bind _output_get_2 (Variables|Default|SetRotate 5.0))
                (bind (_outhit_2 _returnvalue_7) (Collision|LineTraceForObjects _returnvalue_3 (+ _returnvalue_3 (* (Math|Vector|RotateVector (Math|Vector|GetForwardVector End) (Math|Rotator|MakeRotator 0.0 0.0 _output_get_2)) (Variables|Default|GetDistanse))) (Utilities|Array|MakeArray "ObjectTypeQuery1" "ObjectTypeQuery2" "ObjectTypeQuery4") false 0 "None"))
                (if _returnvalue_7
                  (LocalVariables|SetLine1 (.distance _outhit_2))
                  (bind _output_get_3 (Variables|Default|SetRotate -5.0))
                  (bind (_outhit_3 _returnvalue_8) (Collision|LineTraceForObjects _returnvalue_2 (+ _returnvalue_2 (* (Math|Vector|RotateVector (Math|Vector|GetForwardVector End) (Math|Rotator|MakeRotator 0.0 0.0 _output_get_3)) (Variables|Default|GetDistanse))) (Utilities|Array|MakeArray "ObjectTypeQuery1" "ObjectTypeQuery2" "ObjectTypeQuery4") false 0 "None"))
                  (if _returnvalue_8
                    (LocalVariables|SetLine2 (.distance _outhit_3))
                    (if (> (LocalVariables|GetLine1) (LocalVariables|GetLine2))
                      (Transformation|SetActorRotation (Math|Rotator|MakeRotator (.roll _returnvalue_5) (.pitch _returnvalue_5) (+ (.yaw _returnvalue_5) 5.0)) :!label _label)
                      (else
                        (Transformation|SetActorRotation (Math|Rotator|MakeRotator (.roll _returnvalue_4) (.pitch _returnvalue_4) (+ (.yaw _returnvalue_4) -5.0)) :!label _label_2)))
                    (else
                      (goto _label_2)))
                  (else
                    (goto _label)))))
            (else
              (Transformation|SetActorLocation (+ (Transformation|GetActorLocation self) (* (Math|Vector|GetForwardVector (Variables|Default|GetArrow)) (Variables|Default|GetSpeed))) false false))))))))