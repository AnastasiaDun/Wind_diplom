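; BP_WindZone is a box-shaped zone that repeatedly spawns moving wind actors.
; Shortly after BeginPlay, if the PointSpawn array has entries, it spawns a BP_Wind at each point's transform, copying that point's strength, distance, radius and speed.
; The spawn event re-calls itself after DelaySpawn, looping indefinitely.
; The box, sized in construction and at BeginPlay, destroys any BP_Wind that leaves it, bounding the wind to the zone.
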(event OnComponentEndOverlap(Box)
  (params (OverlappedComponent :type Primitive%20Component%20Object%20Reference) (OtherActor :type Actor%20Object%20Reference) (OtherComp :type Primitive%20Component%20Object%20Reference) (OtherBodyIndex :type Integer))
  (if (== (Utilities|GetClass OtherActor) "/Game/BluePrints/BP_Wind.BP_Wind_C")
    (Actor|DestroyActor OtherActor)))

(event Custom|Spawn
  (for _array_element (Variables|Default|GetPointSpawn)
    (bind _returnvalue (Game|SpawnActorfromClass "/Game/BluePrints/BP_Wind.BP_Wind_C" (Math|Transform|MakeTransform (.location (Transformation|GetActorTransform _array_element)) (.rotation (Transformation|GetActorTransform _array_element)) "1,1,1") "Undefined" 0 0))
    (Variables|/Game/BluePrints/BP_Wind.BP_Wind_C|SetWindStrength _returnvalue (Variables|/Game/BluePrints/Debag/BP_SpawnPoint.BP_SpawnPoint_C|GetWindStrength _array_element))
    (Variables|/Game/BluePrints/BP_Wind.BP_Wind_C|SetDistanse _returnvalue (Variables|/Game/BluePrints/Debag/BP_SpawnPoint.BP_SpawnPoint_C|GetDistance _array_element))
    (Variables|/Game/BluePrints/BP_Wind.BP_Wind_C|SetIn%20Sphere%20Radius _returnvalue (Variables|/Game/BluePrints/Debag/BP_SpawnPoint.BP_SpawnPoint_C|GetSphereRadius _array_element))
    (Variables|/Game/BluePrints/BP_Wind.BP_Wind_C|SetSpeed _returnvalue (Variables|/Game/BluePrints/Debag/BP_SpawnPoint.BP_SpawnPoint_C|GetSpeed _array_element)))
  (Utilities|FlowControl|Delay (Variables|Default|GetDelaySpawn))
  (CallFunction|Spawn))

(event EventBeginPlay
  (Components|Box|SetBoxExtent (Variables|Default|GetBox) (Variables|Default|GetIn%20Box%20Extent) true)
  (Utilities|FlowControl|Delay 1.0)
  (if (Utilities|Array|IsValidIndex (Variables|Default|GetPointSpawn))
    (CallFunction|Spawn)))

(fn ConstructionScript
  (Components|Box|SetBoxExtent (Variables|Default|GetBox) (Variables|Default|GetIn%20Box%20Extent) true))