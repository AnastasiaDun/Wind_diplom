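; Water actor whose mesh receives wind direction and strength through Custom Primitive Data, presumably for its material.
; Construction and BeginPlay write default values to that data.
; Activate stores a wind object and enables Tick, which writes the negated forward vector of the wind's arrow and its scaled strength to the mesh.
; Deactivate stops Tick and calls Reset, which is empty, as are the WindWave start and stop events.
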(event Custom|WindWaveStart
  (params (Wind :type BP%20Wind%20Object%20Reference) (WindSrength :type Float%20%28single-precision%29)))

(event Custom|WindWaveStop)

(event EventBeginPlay
  (Rendering|Material|SetCustomPrimitiveDataVector4 (Variables|Debug|GetStaticMeshComponent) 0 (Math|Vector4|MakeVector4 1.0 1.0 0.0 0.01)))

(event EventActivate
  (params (WindObject :type BP%20Wind%20Object%20Reference) (WindStrength :type Float%20%28single-precision%29))
  (Actor|Tick|SetActorTickEnabled true)
  (Variables|Default|SetWind WindObject)
  (Variables|Default|SetWindStrength WindStrength))

(event EventTick
  (params (DeltaSeconds :type Float%20%28single-precision%29))
  (bind _wind (Variables|Default|GetWind))
  (bind _arrow (Variables|/Game/BluePrints/BP_Wind.BP_Wind_C|GetArrow _wind))
  (bind _returnvalue (Math|Vector|GetForwardVector _arrow))
  (Rendering|Material|SetCustomPrimitiveDataVector4 (Variables|Debug|GetStaticMeshComponent) 0 (Math|Vector4|MakeVector4 (* -1 (.x _returnvalue)) (* -1 (.y _returnvalue)) 0.0 (* 40 (Variables|/Game/BluePrints/BP_Wind.BP_Wind_C|GetWindStrength _wind)))))

(event EventDeactivate
  (Actor|Tick|SetActorTickEnabled false)
  (CallFunction|Reset))

(fn ConstructionScript
  (Rendering|Material|SetCustomPrimitiveDataVector4 (Variables|Debug|GetStaticMeshComponent) 0 (Math|Vector4|MakeVector4 1.0 1.0 0.0 0.01)))

(fn Reset)