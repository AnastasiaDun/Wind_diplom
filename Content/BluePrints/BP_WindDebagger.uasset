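; BP_WindDebagger is a debug actor that shows a wind actor's direction and strength with an arrow.
; Activate stores the wind actor and strength and enables Tick, which copies the wind's rotation onto the debugger.
; A DoOnce on Tick plays a timeline that grows the arrow's X scale from zero to the wind strength.
; Deactivate disables Tick and resets the DoOnce so the growth can replay.
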(event Custom|Activate
  (params (Wind :type BP%20Wind%20Object%20Reference) (WindSrength :type Float%20%28single-precision%29))
  (Actor|Tick|SetActorTickEnabled true)
  (Variables|Default|SetWind Wind)
  (Variables|Default|SetWindStrength WindSrength))

(event Custom|Deactivate
  (Actor|Tick|SetActorTickEnabled false)
  (CallFunction|Reset))

(event Custom|Reset
  (Utilities|FlowControl|DoOnce false) ; enters at Reset
)

(event EventBeginPlay
  (bind _arrow (Variables|Default|GetArrow))
  (Components|Arrow|SetArrowColor(LinearColor) _arrow (Variables|Default|GetLine%20Color))
  (Transformation|SetWorldScale3D _arrow "0.000000,2.000000,2.000000"))

(event EventTick
  (params (DeltaSeconds :type Float%20%28single-precision%29))
  (Utilities|FlowControl|Sequence
    (:then_0
      (Utilities|FlowControl|DoOnce false
        (:Completed
          (bind _newtrack_0 (Timeline|Line PlayFromStart)
            (:Update
              (Transformation|SetWorldScale3D (Variables|Default|GetArrow) (Math|Vector|MakeVector (Math|Float|Lerp 0.0 (* 1 (Variables|Default|GetWindStrength)) _newtrack_0) 2.0 2.0)))))))
    (:then_1
      (Transformation|SetActorRotation self (Transformation|GetActorRotation (Variables|Default|GetWind))))))

(fn ConstructionScript)