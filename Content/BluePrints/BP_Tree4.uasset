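; BP_Tree4 is a birch tree actor that reacts to a wind object passed in through Activate.
; It writes the wind arrow's X/Y direction and strength into the mesh's default custom primitive data, presumably for material-driven sway.
; On first activation a timeline ramps strength up from zero; later ones use a second timeline to blend from the last saved direction to the current one.
; Activate and Deactivate also toggle actor tick.
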(event Custom|Reset
  (bind _wind (Variables|Default|GetWind))
  (bind _arrow (Variables|/Game/BluePrints/BP_Wind.BP_Wind_C|GetArrow _wind))
  (bind _returnvalue (Math|Vector|GetForwardVector _arrow))
  (Utilities|FlowControl|DoOnce false) ; enters at Reset
)

(event Custom|WindCollision
  (bind _wind (Variables|Default|GetWind))
  (bind _arrow (Variables|/Game/BluePrints/BP_Wind.BP_Wind_C|GetArrow _wind))
  (bind _returnvalue (Math|Vector|GetForwardVector _arrow))
  (bind _newtrack_0 (Timeline|Timeline_0 PlayFromStart)
    (:Update
      (Rendering|Material|SetDefaultCustomPrimitiveDataVector4 (Variables|Default|GetSM_TreeBirch_01) 0 (Math|Vector4|MakeVector4 (.x _returnvalue) (.y _returnvalue) 0.0 (Math|Float|Lerp 0.0 (Variables|Default|GetWindStrength) _newtrack_0))))
    (:Finished
      (Variables|Default|SetFirst false)
      (Variables|Default|SetA (.x _returnvalue))
      (Variables|Default|SetA_0 (.y _returnvalue)))))

(event Custom|WindSecondCollision
  (bind _wind (Variables|Default|GetWind))
  (bind _arrow (Variables|/Game/BluePrints/BP_Wind.BP_Wind_C|GetArrow _wind))
  (bind _returnvalue (Math|Vector|GetForwardVector _arrow))
  (bind _newtrack_0 (Timeline|Timeline_1 PlayFromStart)
    (:Update
      (Rendering|Material|SetDefaultCustomPrimitiveDataVector4 (Variables|Default|GetSM_TreeBirch_01) 0 (Math|Vector4|MakeVector4 (Math|Float|Lerp (Variables|Default|GetA) (.x _returnvalue) _newtrack_0) (Math|Float|Lerp (Variables|Default|GetA_0) (.y _returnvalue) _newtrack_0) 0.0 (Variables|/Game/BluePrints/BP_Wind.BP_Wind_C|GetWindStrength _wind))))
    (:Finished
      (Variables|Default|SetA (.x _returnvalue))
      (Variables|Default|SetA_0 (.y _returnvalue)))))

(event EventActivate
  (params (WindObject :type BP%20Wind%20Object%20Reference) (WindStrength :type Float%20%28single-precision%29))
  (Actor|Tick|SetActorTickEnabled true)
  (Variables|Default|SetWind WindObject)
  (Variables|Default|SetWindStrength WindStrength)
  (CallFunction|Reset)
  (if (Variables|Default|GetFirst)
    (CallFunction|WindCollision)
    (else
      (CallFunction|WindSecondCollision))))

(event EventDeactivate
  (Actor|Tick|SetActorTickEnabled false))

(fn ConstructionScript)