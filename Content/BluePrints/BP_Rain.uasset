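; BP_Rain is a rain actor that angles its NSRain effect to match a wind actor.
; When an actor of exactly class BP_Wind begins overlapping its Box, it stores that actor, whose world rotation Tick copies to NSRain's relative rotation.
; Activate and Deactivate switch Tick on and off.
; Activate also stores a WindObject, but the rotation update uses only the overlapped actor.
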(event OnComponentBeginOverlap(Box)
  (params (OverlappedComponent :type Primitive%20Component%20Object%20Reference) (OtherActor :type Actor%20Object%20Reference) (OtherComp :type Primitive%20Component%20Object%20Reference) (OtherBodyIndex :type Integer) (bFromSweep :type Boolean) (SweepResult :type Hit%20Result%20Structure%20%28by%20ref%29))
  (if (== (Utilities|GetClass OtherActor) "/Game/BluePrints/BP_Wind.BP_Wind_C")
    (Variables|Default|SetOther%20Actor OtherActor)))

(event EventTick
  (params (DeltaSeconds :type Float%20%28single-precision%29))
  (Transformation|SetRelativeRotation (Variables|Default|GetNS_Rain) (Transformation|GetActorRotation (Variables|Default|GetOther%20Actor)) false false))

(event EventActivate
  (params (WindObject :type BP%20Wind%20Object%20Reference) (WindStrength :type Float%20%28single-precision%29))
  (Actor|Tick|SetActorTickEnabled true)
  (Variables|Default|SetWind%20Object WindObject))

(event EventDeactivate
  (Actor|Tick|SetActorTickEnabled false))

(fn ConstructionScript)