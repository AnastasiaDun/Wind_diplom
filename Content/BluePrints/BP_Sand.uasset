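; Sand actor whose plane receives live wind data, presumably for a sand material effect.
; WindSandStart stores the wind source and enables Tick; WindSandStop disables it and calls Reset, which is empty.
; Tick writes the negated wind arrow direction and scaled strength into the plane's custom primitive data.
; Strength is read live from the wind actor, so the stored WindStrength copy is unused here.
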(event Custom|WindSandStart
  (params (Wind :type BP%20Wind%20Object%20Reference) (WindSrength :type Float%20%28single-precision%29))
  (Actor|Tick|SetActorTickEnabled true)
  (Variables|Default|SetWind Wind)
  (Variables|Default|SetWindStrength WindSrength))

(event Custom|WindSandStop
  (Actor|Tick|SetActorTickEnabled false)
  (CallFunction|Reset))

(event EventTick
  (params (DeltaSeconds :type Float%20%28single-precision%29))
  (bind _wind (Variables|Default|GetWind))
  (bind _arrow (Variables|/Game/BluePrints/BP_Wind.BP_Wind_C|GetArrow _wind))
  (bind _returnvalue (Math|Vector|GetForwardVector _arrow))
  (Rendering|Material|SetDefaultCustomPrimitiveDataVector4 (Variables|Default|GetPlane) 0 (Math|Vector4|MakeVector4 (* -1 (.x _returnvalue)) (* -1 (.y _returnvalue)) 0.0 (* (Variables|/Game/BluePrints/BP_Wind.BP_Wind_C|GetWindStrength _wind) 0.133))))

(fn ConstructionScript)

(fn Reset)