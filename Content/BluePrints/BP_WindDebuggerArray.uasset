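; BP_WindDebuggerArray is a placeable actor that fills an area with a grid of BP_WindDebagger actors, apparently for debugging wind.
; On BeginPlay it stores its root's world location as the grid origin and calls SpawnDebuggers.
; Nested loops over Ox and Oy spawn the debuggers along world X and Y, spaced by Interval, all at the origin's height.
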(event Custom|SpawnDebuggers
  (bind _location (Variables|Default|GetLocation))
  (for _index (range 0 (Variables|Default|GetOx))
    (for _index_2 (range 0 (Variables|Default|GetOy))
      (Game|SpawnActorfromClass "/Game/BluePrints/BP_WindDebagger.BP_WindDebagger_C" (Math|Transform|MakeTransform (Math|Vector|MakeVector (+ (* _index (Variables|Default|GetInterval)) (.x _location)) (+ (* _index_2 (Variables|Default|GetInterval)) (.y _location)) (.z _location)) "0, 0, 0" "1,1,1") "Undefined" 0 0))))

(event EventBeginPlay
  (Variables|Default|SetLocation (Transformation|GetWorldLocation (Variables|Default|GetDefaultSceneRoot)))
  (CallFunction|SpawnDebuggers))

(fn ConstructionScript)