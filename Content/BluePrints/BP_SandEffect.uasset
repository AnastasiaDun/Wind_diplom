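; BP_SandEffect is an actor that drives a sand effect, FXSand, whose orientation follows a wind object.
; Activate stores the supplied WindObject, enables actor tick and activates FXSand.
; While ticking, it copies the wind object's rotation to FXSand's world rotation each frame.
; Deactivate disables tick, stopping the rotation updates, and calls Activate on FXSand with reset set to false.
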(event EventActivate
  (params (WindObject :type BP%20Wind%20Object%20Reference) (WindStrength :type Float%20%28single-precision%29))
  (Variables|Default|SetWind%20Object WindObject)
  (Actor|Tick|SetActorTickEnabled true)
  (Components|Activation|Activate (Variables|Default|GetFX_Sand) true))

(event EventDeactivate
  (Actor|Tick|SetActorTickEnabled false)
  (Components|Activation|Activate (Variables|Default|GetFX_Sand) false))

(event EventTick
  (params (DeltaSeconds :type Float%20%28single-precision%29))
  (Transformation|SetWorldRotation (Variables|Default|GetFX_Sand) (Transformation|GetActorRotation (Variables|Default|GetWind%20Object)) false false))

(fn ConstructionScript)