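; BP_Cloth is an actor that positions a wind source according to a wind object's rotation, apparently to drive cloth movement.
; Activate stores the given WindObject and enables tick; Deactivate disables it.
; Each tick copies the wind object's rotation to the Arrow's relative rotation and moves WindSourse to the Sphere's location, which BeginPlay also sets.
; The box overlap handler is empty, and a debug print event remains.
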(event OnComponentBeginOverlap(Box)
  (params (OverlappedComponent :type Primitive%20Component%20Object%20Reference) (OtherActor :type Actor%20Object%20Reference) (OtherComp :type Primitive%20Component%20Object%20Reference) (OtherBodyIndex :type Integer) (bFromSweep :type Boolean) (SweepResult :type Hit%20Result%20Structure%20%28by%20ref%29)))

(event Custom|zalupa
  (Development|PrintString "Hello"))

(event EventBeginPlay
  (Transformation|SetActorLocation (Variables|Default|GetWindSourse) (Transformation|GetWorldLocation (Variables|Default|GetSphere)) false false))

(event EventActivate
  (params (WindObject :type BP%20Wind%20Object%20Reference) (WindStrength :type Float%20%28single-precision%29))
  (Actor|Tick|SetActorTickEnabled true)
  (Variables|Default|SetWind%20Object WindObject))

(event EventDeactivate
  (Actor|Tick|SetActorTickEnabled false))

(event EventTick
  (params (DeltaSeconds :type Float%20%28single-precision%29))
  (Transformation|SetRelativeRotation (Variables|Default|GetArrow) (Transformation|GetActorRotation (Variables|Default|GetWind%20Object)) false false)
  (Transformation|SetActorLocation (Variables|Default|GetWindSourse) (Transformation|GetWorldLocation (Variables|Default|GetSphere)) false false))

(fn ConstructionScript)