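; BP_Tree is a tree actor that passes wind direction and strength to its cylinder mesh while wind affects it.
; WindTreeStart stores the wind source and enables Tick; WindTreeSrop disables Tick and calls Reset, which is currently empty.
; Each Tick writes the wind arrow's forward X/Y and the source's strength into Custom Primitive Data, exposing them to materials per primitive.
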(event Custom|WindTreeStart
  (params (Wind :type BP%20Wind%20Object%20Reference) (WindSrength :type Float%20%28single-precision%29))
  (Actor|Tick|SetActorTickEnabled true)
  (Variables|Default|SetWind Wind)
  (Variables|Default|SetWindStrength WindSrength))

(event Custom|WindTreeSrop
  (Actor|Tick|SetActorTickEnabled false)
  (CallFunction|Reset))

(event EventTick
  (params (DeltaSeconds :type Float%20%28single-precision%29))
  (bind _wind (Variables|Default|GetWind))
  (bind _arrow (Variables|/Game/BluePrints/BP_Wind.BP_Wind_C|GetArrow _wind))
  (bind _returnvalue (Math|Vector|GetForwardVector _arrow))
  (Rendering|Material|SetDefaultCustomPrimitiveDataVector4 (Variables|Default|GetCylinder) 0 (Math|Vector4|MakeVector4 (.x _returnvalue) (.y _returnvalue) 0.0 (Variables|/Game/BluePrints/BP_Wind.BP_Wind_C|GetWindStrength _wind))))

(fn ConstructionScript)

(fn Reset)