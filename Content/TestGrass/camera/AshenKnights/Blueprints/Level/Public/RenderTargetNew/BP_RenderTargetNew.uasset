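; Scene capture actor that follows the player to maintain a persistent render target of the area around them.
; Each tick it snaps XY to a 1/512 texel grid of the ortho width to avoid jitter and sits one ortho width below the player.
; It publishes capture location and size to material parameters, then draws M_DrawToPersistent with the normalized move offset to scroll accumulated data.
; BeginPlay clears both render targets.
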(event EventBeginPlay
  ;[1 1 1] CaptureSizeStorage
  (Rendering|Material|SetScalarParameterValue "/Game/TestGrass/AshenKnights/Materials/ParameterCollections/MPC_RenderTargetStorage.MPC_RenderTargetStorage" "CaptureSize" (Variables|/Script/Engine.SceneCaptureComponent2D|GetOrthoWidth (Variables|Default|GetSceneCaptureComponent2D)) :!class /Script/Engine.KismetMaterialLibrary)
  ;[1 1 1] CreateDynamicMaterial_Inst
  (bind _returnvalue (Rendering|Material|CreateDynamicMaterialInstance "/Game/TestGrass/camera/AshenKnights/Materials/MasterMaterials/RenderTarget/M_DrawToPersistent.M_DrawToPersistent" "None" "None" :!class /Script/Engine.KismetMaterialLibrary))
  (Variables|Default|SetDrawMatiral _returnvalue)
  ;[1 1 1] ClearOldRenderTargetInfo
  (Rendering|ClearRenderTarget2D "/Game/TestGrass/AshenKnights/Materials/RenderTarget/RT_Capture.RT_Capture")
  (Rendering|ClearRenderTarget2D "/Game/TestGrass/camera/AshenKnights/Materials/RenderTarget/RT_Persistent.RT_Persistent"))

(event Collision|EventActorBeginOverlap
  (params (OtherActor :type Actor%20Object%20Reference)))

(event EventTick
  (params (DeltaSeconds :type Float%20%28single-precision%29))
  (Utilities|IsValid (Game|GetPlayerCharacter 0)
    (:Is%20Valid
      (CallFunction|CaptureOffset)
      (CallFunction|CameraLocationStorage)
      (CallFunction|DrawtoPersistent))))

(fn ConstructionScript)

(fn DrawtoPersistent
  (bind _scenecapturecomponent2d (Variables|Default|GetSceneCaptureComponent2D))
  (bind _moveoffset (Variables|Default|GetMoveOffset))
  (bind _orthowidth (Variables|/Script/Engine.SceneCaptureComponent2D|GetOrthoWidth _scenecapturecomponent2d))
  (bind _returnvalue (/ _moveoffset _orthowidth))
  (Rendering|Material|SetVectorParameterValue (Variables|Default|GetDrawMatiral) "Offset" (Utilities|Struct|MakeLinearColor (.x _returnvalue) (.y _returnvalue) 0.0 1.0) :!class /Script/Engine.MaterialInstanceDynamic)
  (Rendering|DrawMaterialtoRenderTarget 0 (Variables|Default|GetDrawMatiral)))

(fn CaptureOffset
  (bind _returnvalue (/ 1.0 512.0))
  (bind _returnvalue_2 (Transformation|GetActorLocation))
  (bind _returnvalue_3 (Game|GetPlayerCharacter 0))
  (bind _scenecapturecomponent2d (Variables|Default|GetSceneCaptureComponent2D))
  (bind _returnvalue_4 (Transformation|GetActorLocation _returnvalue_3))
  (bind _orthowidth (Variables|/Script/Engine.SceneCaptureComponent2D|GetOrthoWidth _scenecapturecomponent2d))
  (bind _returnvalue_5 (* _orthowidth _returnvalue))
  (bind _returnvalue_6 (/ (Math|Vector2D|MakeVector2D (.x _returnvalue_4) (.y _returnvalue_4)) _returnvalue_5))
  (bind _returnvalue_7 (+ _returnvalue_6 0.5))
  (bind _output_get (Variables|Default|SetMoveOffset (- (* (Math|Vector2D|MakeVector2D (Math|Conversions|ToFloat(Integer) (Math|Float|Floor (.x _returnvalue_7))) (Math|Conversions|ToFloat(Integer) (Math|Float|Floor (.y _returnvalue_7)))) _returnvalue_5) (Math|Vector2D|MakeVector2D (.x _returnvalue_2) (.y _returnvalue_2)))))
  (Transformation|AddActorWorldOffset (Math|Vector|MakeVector (.x _output_get) (.y _output_get) (- (- (.z (Transformation|GetActorLocation (Game|GetPlayerCharacter 0))) (.z (Transformation|GetActorLocation))) (Variables|/Script/Engine.SceneCaptureComponent2D|GetOrthoWidth (Variables|Default|GetSceneCaptureComponent2D))))))

(fn CameraLocationStorage
  (Rendering|Material|SetVectorParameterValue 0 "CaptureLocation" (Math|Conversions|ToLinearColor(Vector) (Transformation|GetActorLocation)) :!class /Script/Engine.KismetMaterialLibrary))